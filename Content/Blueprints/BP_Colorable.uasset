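; BP_Colorable is a Blueprint that displays a configurable static mesh tinted with the first entry of its Colors array.
; Both the construction script and BeginPlay assign Mesh to ColorableMesh, create a dynamic material instance on element 0 and set its BaseColor parameter.
; BeginPlay also stores that first color as CurrentColor, though the graphs shown contain no logic for switching to other colors.
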(event `self.ReceiveBeginPlay`
  (bind _output (`|GetArrayItem` (`self.Colors`)))
  (`StaticMeshComponent.SetStaticMesh` (`self.ColorableMesh`) (`self.Mesh`))
  (bind _returnvalue (`PrimitiveComponent.CreateDynamicMaterialInstance` (`self.ColorableMesh`) 0 null))
  (set `self.DynaMat` _returnvalue)
  (`MaterialInstanceDynamic.SetVectorParameterValue` (`self.DynaMat`) "BaseColor" _output)
  (set `self.CurrentColor` _output))

(fn `UserConstructionScript`
  (`StaticMeshComponent.SetStaticMesh` (`self.ColorableMesh`) (`self.Mesh`))
  (bind _returnvalue (`PrimitiveComponent.CreateDynamicMaterialInstance` (`self.ColorableMesh`) 0 null))
  (set `self.DynaMat` _returnvalue)
  (`MaterialInstanceDynamic.SetVectorParameterValue` (`self.DynaMat`) "BaseColor" (`|GetArrayItem` (`self.Colors`))))