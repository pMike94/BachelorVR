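; BP_MenuBase is a radial color menu for BP_Colorable actors, operated with motion controllers.
; On BeginPlay it scales in via timeline, then spawns one indexed BP_MenuButton child actor per color of the targeted colorable, evenly rotated around roll.
; Motion controller overlap on its Cylinder toggles an Overlapped flag and custom-depth highlight.
; ClearMenu untargets and unhighlights all colorables, then destroys the menu.
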(event `self.ReceiveBeginPlay`
  (bind _colors (`/Game/Blueprints/BP_Colorable.Colors` (`self.Target`)))
  (bind (_direction _newtrack_0) (`Timeline|TL_MenuBase` :!via `PlayFromStart`)
    (:`Update`
      (`self.SetActorScale3D` (`KismetMathLibrary.Conv_DoubleToVector` _newtrack_0)))
    (:`Finished`
      (bind _outactors (`GameplayStatics.GetAllActorsOfClass` "/Game/Blueprints/BP_Colorable.BP_Colorable_C"))
      (for _array_element _outactors
        (if (`/Game/Blueprints/BP_Colorable.Targeted` _array_element)
          (set `self.Target` _array_element)))
      (for (_ _array_index) _colors
        (bind _returnvalue (`AddComponent|NODE_AddChildActorComponent-1`))
        (`SceneComponent.K2_SetRelativeRotation` _returnvalue (`KismetMathLibrary.MakeRotator` (* (`KismetMathLibrary.Conv_IntToDouble` _array_index) (/ 360.0 (`KismetMathLibrary.Conv_IntToDouble` (`KismetArrayLibrary.Array_Length` _colors))))) false false)
        (`ChildActorComponent.SetChildActorClass` _returnvalue "/Game/Blueprints/BP_MenuButton.BP_MenuButton_C")
        (bind _asbp_menu_button (cast `/Game/Blueprints/BP_MenuButton` (`ChildActorComponent.ChildActor` _returnvalue)))
        (set `/Game/Blueprints/BP_MenuButton.ID` _array_index _asbp_menu_button)))))

(event `self.Cylinder.OnComponentBeginOverlap`
  (params (OverlappedComponent :type "PrimitiveComponent Object Reference") (OtherActor :type "Actor Object Reference") (OtherComp :type "PrimitiveComponent Object Reference") (OtherBodyIndex :type Integer) (bFromSweep :type Boolean) (SweepResult :type "HitResult Structure (by ref)"))
  ;[1 1 1] Activate Button
  (cast `/Game/VirtualRealityBP/Blueprints/BP_MotionController` OtherActor)
  (`PrimitiveComponent.SetRenderCustomDepth` (`self.Cylinder`) true)
  (set `self.Overlapped` true))

(event `self.Cylinder.OnComponentEndOverlap`
  (params (OverlappedComponent :type "PrimitiveComponent Object Reference") (OtherActor :type "Actor Object Reference") (OtherComp :type "PrimitiveComponent Object Reference") (OtherBodyIndex :type Integer))
  ;[1 1 1] Deactivate Button
  (cast `/Game/VirtualRealityBP/Blueprints/BP_MotionController` OtherActor)
  (`PrimitiveComponent.SetRenderCustomDepth` (`self.Cylinder`) false)
  (set `self.Overlapped` false))

(fn `ClearMenu`
  (bind _outactors (`GameplayStatics.GetAllActorsOfClass` "/Game/Blueprints/BP_Colorable.BP_Colorable_C"))
  (for _array_element _outactors
    (set `/Game/Blueprints/BP_Colorable.Targeted` false _array_element)
    (`PrimitiveComponent.SetRenderCustomDepth` (`/Game/Blueprints/BP_Colorable.ColorableMesh` _array_element) false))
  (`self.K2_DestroyActor`))

(fn `UserConstructionScript`)