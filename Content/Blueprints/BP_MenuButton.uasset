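; BP_MenuButton is a VR menu button that applies a color to the furniture targeted by BP_MenuBase.
; On BeginPlay it takes its color from the target's Colors by ID, tints its own cylinder and animates scale and height with a timeline.
; Motion controller overlap toggles an outline via custom depth and the Overlapped flag.
; ButtonInteract sets the target's material color and picks the standard texture for ID zero, otherwise the colored one.
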(event `self.ReceiveBeginPlay`
  (bind _scene (`self.Scene`))
  ;[1 1 1] Init Delay
  (`KismetSystemLibrary.Delay` 0.02)
  ;[1 1 1] Dynamic Material Instance
  (bind _returnvalue (`PrimitiveComponent.CreateDynamicMaterialInstance` (`self.Cylinder`) 0 null))
  (set `self.DynaMat` _returnvalue)
  ;[1 1 1] Get Targeted Furniture and "Color from ID"
  (bind _outactors (`GameplayStatics.GetAllActorsOfClass` "/Game/Blueprints/BP_MenuBase.BP_MenuBase_C"))
  (bind _target (`/Game/Blueprints/BP_MenuBase.Target` (`|GetArrayItem` _outactors)))
  (set `self.Target` _target)
  (bind _output (`|GetArrayItem` (`/Game/Blueprints/BP_Colorable.Colors` _target) (`self.ID`)))
  (set `self.Color` _output)
  (`MaterialInstanceDynamic.SetVectorParameterValue` (`self.DynaMat`) "BaseColor" _output)
  (bind (_direction _scale _positionz) (`Timeline|Timeline_0` :!via `PlayFromStart`)
    (:`Update`
      (`SceneComponent.SetRelativeScale3D` _scene (`KismetMathLibrary.Conv_DoubleToVector` _scale))
      (`SceneComponent.K2_SetRelativeLocation` _scene (`KismetMathLibrary.MakeVector` 0.0 0.0 (* _positionz 40.0)) false false))))

(event `self.Cylinder.OnComponentBeginOverlap`
  (params (OverlappedComponent :type "PrimitiveComponent Object Reference") (OtherActor :type "Actor Object Reference") (OtherComp :type "PrimitiveComponent Object Reference") (OtherBodyIndex :type Integer) (bFromSweep :type Boolean) (SweepResult :type "HitResult Structure (by ref)"))
  ;[1 1 1] Activate Button
  (cast `/Game/VirtualRealityBP/Blueprints/BP_MotionController` OtherActor)
  (`PrimitiveComponent.SetRenderCustomDepth` (`self.Cylinder`) true)
  (set `self.Overlapped` true))

(event `ButtonInteract`
  (bind _target (`self.Target`))
  (bind _target_2 (`self.Target`))
  ;[1 1 1] Set Color
  (`MaterialInstanceDynamic.SetVectorParameterValue` (`/Game/Blueprints/BP_Colorable.DynaMat` (`self.Target`)) "BaseColor" (`self.Color`))
  (if (== (`self.ID`) 0)
    (`MaterialInstanceDynamic.SetTextureParameterValue` (`/Game/Blueprints/BP_Colorable.DynaMat` _target_2) "BaseTexture" (`/Game/Blueprints/BP_Colorable.StandardTexture` _target_2))
    (else
      (`MaterialInstanceDynamic.SetTextureParameterValue` (`/Game/Blueprints/BP_Colorable.DynaMat` _target) "BaseTexture" (`/Game/Blueprints/BP_Colorable.ColoredTexture` _target)))))

(event `self.Cylinder.OnComponentEndOverlap`
  (params (OverlappedComponent :type "PrimitiveComponent Object Reference") (OtherActor :type "Actor Object Reference") (OtherComp :type "PrimitiveComponent Object Reference") (OtherBodyIndex :type Integer))
  ;[1 1 1] Deactivate Button
  (cast `/Game/VirtualRealityBP/Blueprints/BP_MotionController` OtherActor)
  (`PrimitiveComponent.SetRenderCustomDepth` (`self.Cylinder`) false)
  (set `self.Overlapped` false))

(fn `UserConstructionScript`)